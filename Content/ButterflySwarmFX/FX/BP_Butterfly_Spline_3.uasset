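; Butterfly swarm effect Blueprint that moves a Niagara component along a spline path.
; Each Tick advances a distance value scaled by frame time and Speed, then sets the Niagara component's world location to a point sampled along the spline.
; When the distance passes the spline's end it resets to zero, so the effect repeats the path continuously.
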(event `self.ReceiveTick`
  (params (DeltaSeconds :type "Float (single-precision)"))
  (bind _spline (`self.Spline`))
  (bind _returnvalue (+ (* (* DeltaSeconds 25.0) (`self.Speed`)) (`self.Distance`)))
  ;[1 1 1] Loop the spline
  (set `self.Distance` _returnvalue)
  (`SceneComponent.K2_SetWorldLocation` (`self.Niagara`) (`SplineComponent.GetLocationAtDistanceAlongSpline` _spline _returnvalue "World") false false)
  (`/Engine/EditorBlueprintResources/StandardMacros.CompareFloat` (`self.Distance`) (`SplineComponent.GetDistanceAlongSplineAtSplinePoint` _spline (`SplineComponent.GetNumberOfSplinePoints` _spline))
    (:`>`
      (set `self.Distance` 0.0))))

(fn `UserConstructionScript`)