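; Fireworks launcher actor that spawns BP_Fireworks_Rocket actors in timed sequences, with a configurable launcher mesh set in construction.
; While active, Tick checks the delay timer, fires a rocket with random cone direction and speed from its firework data, then advances the sequence.
; Each rocket's firework is random or the current list entry, which cycles after each sequence.
; LaunchMultyRockets and LaunchStop toggle activity; sequences optionally loop.
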(event `self.ReceiveBeginPlay`
  ;[1 1 1] Begin Play
  ;[1 1 1] Initial Settings
  (set `self.InGame` true))

(event `self.ReceiveTick`
  (params (DeltaSeconds :type "Float (single-precision)"))
  ;[1 1 1] Event Tick
  ;[1 1 1] Checking whether it is possible to launch missiles
  (if (and (`self.IsActive`) (`self.Check Launcher Timer`))
    ;[1 1 1] Launch Rocket
    (`self.Launch Single Rocket`)
    ;[1 1 1] Update Sequnce
    (`self.UpdateSequence`)))

(fn `Check Launcher Timer`
  (returns (Can :type Boolean))
  (locals (TempDelayTime :type "Float (double-precision)"))
  ;[1 1 1] 1st rocket
  (if (== (`self.CurrentRocketIndex`) 0)
    (if (`self.IsLooping`)
      ;[1 1 1] >= 2nd loop
      (set `local.TempDelayTime` (`self.Delay Between Sequnces`))
      (else
        ;[1 1 1] 1st loop
        (set `local.TempDelayTime` (`self.Initial Sequence Delay`))))
    (else
      ;[1 1 1] >= 2nd rocket
      (set `local.TempDelayTime` (`self.Delay Between Rockets`))))
  (return (>= (`GameplayStatics.GetTimeSeconds`) (+ (`local.TempDelayTime`) (`self.LastLaunchTime`)))))

(fn `Get Current Firework`
  (returns (DT_Firework :type "/Game/AdvancedFireworks/DATA/PDA_Firework Object Reference"))
  (if (`self.Random/InTurn`)
    (bind _output (`self.Get Random Firework`))
    (return _output)
    (else
      (return (`|GetArrayItem` (`self.DT_Firework`) (`self.CurrentDAIndex`))))))

(fn `Get Random Firework`
  (returns (Output :type "/Game/AdvancedFireworks/DATA/PDA_Firework Object Reference"))
  (bind _dt_firework (`self.DT_Firework`))
  (return (`|GetArrayItem` _dt_firework (`KismetMathLibrary.RandomIntegerInRange` 0 (`KismetArrayLibrary.Array_LastIndex` _dt_firework)))))

(fn `Launch Multy Rockets`
  (if (`self.InGame`)
    (set `self.LastLaunchTime` (`GameplayStatics.GetTimeSeconds`))
    (set `self.IsActive` true)
    (set `self.IsLooping` false)))

(fn `Launch Single Rocket`
  (if (`self.InGame`)
    (bind _dt_firework (`self.Get Current Firework`))
    (bind _returnvalue (`|SpawnActorFromClass` "/Game/AdvancedFireworks/Blueprints/BP_Fireworks_Rocket.BP_Fireworks_Rocket_C" (`KismetMathLibrary.MakeTransform` (+ (`self.K2_GetActorLocation`) (`KismetMathLibrary.TransformDirection` (`self.GetTransform`) (`self.LaunchPosition`))) (`self.K2_GetActorRotation`)) "AlwaysSpawn" "OverrideRootScale" null _dt_firework null))
    (bind (_min_max_launch_angle_x _min_max_launch_angle_y) (`KismetMathLibrary.BreakVector2D` (`/Game/AdvancedFireworks/DATA/PDA_Firework.Min/Max Launch Angle` _dt_firework)))
    (bind (_min_max_rocket_speed_x _min_max_rocket_speed_y) (`KismetMathLibrary.BreakVector2D` (`/Game/AdvancedFireworks/DATA/PDA_Firework.Min/Max Rocket Speed` _dt_firework)))
    (`PrimitiveComponent.SetPhysicsLinearVelocity` (`/Game/AdvancedFireworks/Blueprints/BP_Fireworks_Rocket.Mesh` _returnvalue) (* (`KismetMathLibrary.RandomUnitVectorInConeInDegrees` (`self.GetActorUpVector`) (`KismetMathLibrary.RandomFloatInRange` _min_max_launch_angle_x _min_max_launch_angle_y)) (`KismetMathLibrary.RandomFloatInRange` _min_max_rocket_speed_x _min_max_rocket_speed_y)) false "None")
    (set `self.LastLaunchTime` (`GameplayStatics.GetTimeSeconds`))))

(fn `Launch Stop`
  (set `self.IsActive` false))

(fn `Set Launcher Initial Settings`
  (`StaticMeshComponent.SetStaticMesh` (`self.Mesh`) (`self.LauncherMesh`))
  (`SceneComponent.K2_SetRelativeTransform` (`self.Mesh`) (`self.LauncherTransform`) false true)
  (`SceneComponent.SetVisibility` (`self.Mesh`) (`self.LauncherVisibility`) false))

(fn `UpdateSequence`
  ;[1 1 1] Add Current Rocket Index
  (bind _result (`/Engine/EditorBlueprintResources/StandardMacros.IncrementInt` (`self.CurrentRocketIndex`))
    (:`  `
      (if (< _result (`self.NumOfLaunchRockets`))
        (return)
        (else
          ;[1 1 1] Get Current Data Asset Index
          (if (== (`KismetArrayLibrary.Array_LastIndex` (`self.DT_Firework`)) (`self.CurrentDAIndex`))
            (set `self.CurrentDAIndex` 0)
            (else
              (`/Engine/EditorBlueprintResources/StandardMacros.IncrementInt` (`self.CurrentDAIndex`)
                (:`  `
                  _))))
          ;[1 1 1] Reset Current Rocket Index
          (set `self.CurrentRocketIndex` 0)
          (if (`self.Sequence Loops`)
            (set `self.IsLooping` true)
            (else
              (set `self.IsActive` false)))
          (return))))))

(fn `UserConstructionScript`
  (`self.Set Launcher Initial Settings`))