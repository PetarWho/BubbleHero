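; Firework rocket actor that shows a Niagara rocket and trails, then bursts into explosion effects, all configured by its DTFirework settings.
; Construction randomizes lifespan and styles the rocket sprite through a dynamic material.
; BeginPlay attaches trail systems to the mesh by type.
; Tick deactivates trails after the lifespan and, following a delay, spawns each configured explosion once at the mesh location with randomized parameters.
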(event `self.ReceiveBeginPlay`
  (`self.SetNiagaraTrails`))

(event `self.ReceiveTick`
  (params (DeltaSeconds :type "Float (single-precision)"))
  (bind (_min_max_rocket_lifespan_x _min_max_rocket_lifespan_y) (`KismetMathLibrary.BreakVector2D` (`/Game/AdvancedFireworks/DATA/PDA_Firework.Min/Max Rocket Lifespan` (`self.DT_Firework`))))
  (if (not (`self.IsTrailActive`))
    (bind _output_get (set `self.CurrentLifespan` (`KismetMathLibrary.RandomFloatInRange` _min_max_rocket_lifespan_x _min_max_rocket_lifespan_y))))
  (if (> (`self.GetGameTimeSinceCreation`) _output_get)
    (set `self.IsTrailActive` false)
    (`self.DeactivateTrails`))
  (if (and (> (`self.GetGameTimeSinceCreation`) (+ (`self.CurrentLifespan`) (`/Game/AdvancedFireworks/DATA/PDA_Firework.ExplosionDelay` (`self.DT_Firework`)))) (`self.IsUnexploded`))
    (`self.ExplodeRocket`)
    (set `self.IsUnexploded` false)))

(fn `DeactivateTrails`
  (for _array_element (`self.TrailRefs`)
    (`ActorComponent.Deactivate` _array_element)))

(fn `ExplodeRocket`
  (locals (NSRef :type "NiagaraComponent Object Reference"))
  (for _array_element (`/Game/AdvancedFireworks/DATA/PDA_Firework.ExplosionSettings` (`self.DT_Firework`))
    (bind _output_get (`self.Set Explosion Type` _array_element))
    (bind _returnvalue (`NiagaraFunctionLibrary.SpawnSystemAtLocation` _output_get (`SceneComponent.K2_GetComponentLocation` (`self.Mesh`))))
    (set `local.NSRef` _returnvalue)
    (bind (_start_color _end_color _duration _density _radius _scale _tint_random _type _images _use_image_color) (`self.Get Explosion Info` _array_element))
    (switch `/Game/AdvancedFireworks/DATA/Enums/E_Fireworks_ExplosionType` _type
      (:`NewEnumerator3`
        _)
      (:`NewEnumerator4`
        _)
      (:`NewEnumerator5`
        _)
      (:`NewEnumerator7`
        _)
      (:`NewEnumerator11`
        _)
      (:`NewEnumerator8`
        _)
      (:`NewEnumerator9`
        _)
      (:`NewEnumerator10`
        _)
      (:`NewEnumerator6`
        (`NiagaraComponent.SetVariableTexture` (`local.NSRef`) "ImageTexture" _images)
        (`NiagaraComponent.SetVariableBool` (`local.NSRef`) "UseImageColor" _use_image_color)))
    (`NiagaraComponent.SetVariableFloat` (`local.NSRef`) "Density" _density)
    (`NiagaraComponent.SetVariableFloat` (`local.NSRef`) "Duration" _duration)
    (`NiagaraComponent.SetVariableFloat` (`local.NSRef`) "Radius" _radius)
    (`NiagaraComponent.SetVariableFloat` (`local.NSRef`) "Scale" _scale)
    (`NiagaraComponent.SetVariableFloat` (`local.NSRef`) "HueShift" (`KismetMathLibrary.RandomFloatInRange` 0.0 _tint_random))
    (`NiagaraComponent.SetVariableLinearColor` (`local.NSRef`) "StartColor" _start_color)
    (`NiagaraComponent.SetVariableLinearColor` (`local.NSRef`) "EndColor" _end_color)))

(fn `Get Explosion Info`
  (params (Explosion :type "/Game/AdvancedFireworks/DATA/Structures/S_Firework_Explosion Structure"))
  (returns (`Start Color` :type "LinearColor Structure") (`End Color` :type "LinearColor Structure") (Duration :type "Float (double-precision)") (Density :type "Float (double-precision)") (Radius :type "Float (double-precision)") (Scale :type "Float (double-precision)") (`Tint Random` :type "Float (double-precision)") (Type :type "/Game/AdvancedFireworks/DATA/Enums/E_Fireworks_ExplosionType Enum") (Images :type "Texture2D Object Reference") (`Use Image Color` :type Boolean))
  (bind (_type _minmaxduration _minmaxdensity _minmaxradius _minmaxscale _tintrandom _startcolor _endcolor _images _useimagecolor) (break `/Game/AdvancedFireworks/DATA/Structures/S_Firework_Explosion` Explosion))
  (return _startcolor _endcolor (`KismetMathLibrary.RandomFloatInRange` (`KismetMathLibrary.BreakVector2D` _minmaxduration) (`.Y` (`KismetMathLibrary.BreakVector2D` _minmaxduration))) (`KismetMathLibrary.RandomFloatInRange` (`KismetMathLibrary.BreakVector2D` _minmaxdensity) (`.Y` (`KismetMathLibrary.BreakVector2D` _minmaxdensity))) (`KismetMathLibrary.RandomFloatInRange` (`KismetMathLibrary.BreakVector2D` _minmaxradius) (`.Y` (`KismetMathLibrary.BreakVector2D` _minmaxradius))) (`KismetMathLibrary.RandomFloatInRange` (`KismetMathLibrary.BreakVector2D` _minmaxscale) (`.Y` (`KismetMathLibrary.BreakVector2D` _minmaxscale))) _tintrandom _type (`|GetArrayItem` _images (`KismetMathLibrary.RandomIntegerInRange` 0 (`KismetArrayLibrary.Array_LastIndex` _images))) _useimagecolor))

(fn `Get Trail Info`
  (params (Trail :type "/Game/AdvancedFireworks/DATA/Structures/S_Firework_Trail Structure"))
  (returns (`Start Color` :type "LinearColor Structure") (`End Color` :type "LinearColor Structure") (Density :type "Float (double-precision)") (Length :type "Float (double-precision)") (Scale :type "Float (double-precision)") (`Tint Random` :type "Float (double-precision)"))
  (bind (_type _minmaxdensity _minmaxlength _minmaxscale _tintrandom _startcolor _endcolor) (break `/Game/AdvancedFireworks/DATA/Structures/S_Firework_Trail` Trail))
  (return _startcolor _endcolor (`KismetMathLibrary.RandomFloatInRange` (`KismetMathLibrary.BreakVector2D` _minmaxdensity) (`.Y` (`KismetMathLibrary.BreakVector2D` _minmaxdensity))) (`KismetMathLibrary.RandomFloatInRange` (`KismetMathLibrary.BreakVector2D` _minmaxlength) (`.Y` (`KismetMathLibrary.BreakVector2D` _minmaxlength))) (`KismetMathLibrary.RandomFloatInRange` (`KismetMathLibrary.BreakVector2D` _minmaxscale) (`.Y` (`KismetMathLibrary.BreakVector2D` _minmaxscale))) _tintrandom))

(fn `Set Explosion Type`
  (params (Explosion :type "/Game/AdvancedFireworks/DATA/Structures/S_Firework_Explosion Structure (by ref)"))
  (returns (Output_Get :type "NiagaraSystem Object Reference"))
  (locals (TempNiagaraAsset :type "NiagaraSystem Object Reference"))
  (switch `/Game/AdvancedFireworks/DATA/Enums/E_Fireworks_ExplosionType` (`.Type_20_B87F5B3948B66C142CAE70B5439DA6C5` (break `/Game/AdvancedFireworks/DATA/Structures/S_Firework_Explosion` Explosion))
    (:`NewEnumerator3`
      (return "/Game/AdvancedFireworks/NiagaraVFX/Explosion/NS_Firework_Radial.NS_Firework_Radial"))
    (:`NewEnumerator4`
      (return "/Game/AdvancedFireworks/NiagaraVFX/Explosion/NS_Firework_Disc.NS_Firework_Disc"))
    (:`NewEnumerator5`
      (return "/Game/AdvancedFireworks/NiagaraVFX/Explosion/NS_Firework_Sparkler.NS_Firework_Sparkler"))
    (:`NewEnumerator7`
      (return "/Game/AdvancedFireworks/NiagaraVFX/Explosion/NS_Firework_Ribbons.NS_Firework_Ribbons"))
    (:`NewEnumerator11`
      (return "/Game/AdvancedFireworks/NiagaraVFX/Explosion/NS_Firework_Splash_1.NS_Firework_Splash_1"))
    (:`NewEnumerator8`
      (return "/Game/AdvancedFireworks/NiagaraVFX/Explosion/NS_Firework_Splash_2.NS_Firework_Splash_2"))
    (:`NewEnumerator9`
      (return "/Game/AdvancedFireworks/NiagaraVFX/Explosion/NS_Firework_Tails_1.NS_Firework_Tails_1"))
    (:`NewEnumerator10`
      (return "/Game/AdvancedFireworks/NiagaraVFX/Explosion/NS_Firework_Tails_2.NS_Firework_Tails_2"))
    (:`NewEnumerator6`
      (return "/Game/AdvancedFireworks/NiagaraVFX/Explosion/NS_Firework_Image.NS_Firework_Image"))))

(fn `SetNiagaraTrails`
  (locals (TempNiagaraAsset :type "NiagaraSystem Object Reference") (TrailRef :type "NiagaraComponent Object Reference"))
  (for _array_element (`/Game/AdvancedFireworks/DATA/PDA_Firework.TrailEffects` (`self.DT_Firework`))
    (switch `/Game/AdvancedFireworks/DATA/Enums/E_Fireworks_TrailType` (`.Type_2_B87F5B3948B66C142CAE70B5439DA6C5` (break `/Game/AdvancedFireworks/DATA/Structures/S_Firework_Trail` _array_element))
      (:`NewEnumerator0`
        (set `local.TempNiagaraAsset` "/Game/AdvancedFireworks/NiagaraVFX/Trais/NS_Trail_SimpleSparks.NS_Trail_SimpleSparks"))
      (:`NewEnumerator1`
        (set `local.TempNiagaraAsset` "/Game/AdvancedFireworks/NiagaraVFX/Trais/NS_Trail_Smoke.NS_Trail_Smoke"))
      (:`NewEnumerator2`
        (set `local.TempNiagaraAsset` "/Game/AdvancedFireworks/NiagaraVFX/Trais/NS_Trail_SpiralSparks.NS_Trail_SpiralSparks")))
    (bind _returnvalue (`NiagaraFunctionLibrary.SpawnSystemAttached` (`local.TempNiagaraAsset`) (`self.Mesh`) "None" (0.0 0.0 0.0) (struct) "KeepRelativeOffset"))
    (set `local.TrailRef` _returnvalue)
    (`NiagaraComponent.SetVariableFloat` (`local.TrailRef`) "TrailDuration" (`self.CurrentLifespan`))
    (bind (_start_color _end_color _density _length _scale _tint_random) (`self.Get Trail Info` _array_element))
    (`NiagaraComponent.SetVariableFloat` (`local.TrailRef`) "TrailSpriteScale" _scale)
    (`NiagaraComponent.SetVariableFloat` (`local.TrailRef`) "TrailLengthScale" _length)
    (`NiagaraComponent.SetVariableFloat` (`local.TrailRef`) "TrailDensityScale" _density)
    (`NiagaraComponent.SetVariableFloat` (`local.TrailRef`) "HueShift" (`KismetMathLibrary.RandomFloatInRange` 0.0 _tint_random))
    (`NiagaraComponent.SetVariableLinearColor` (`local.TrailRef`) "StartColor" _start_color)
    (`NiagaraComponent.SetVariableLinearColor` (`local.TrailRef`) "EndColor" _end_color)
    (`KismetArrayLibrary.Array_Add` (`self.TrailRefs`) (`local.TrailRef`))))

(fn `UserConstructionScript`
  (bind _dt_firework (`self.DT_Firework`))
  (bind (_min_max_rocket_lifespan_x _min_max_rocket_lifespan_y) (`KismetMathLibrary.BreakVector2D` (`/Game/AdvancedFireworks/DATA/PDA_Firework.Min/Max Rocket Lifespan` (`self.DT_Firework`))))
  (bind _output_get (set `self.CurrentLifespan` (`KismetMathLibrary.RandomFloatInRange` _min_max_rocket_lifespan_x _min_max_rocket_lifespan_y)))
  (`self.SetLifeSpan` (* (+ _output_get (`/Game/AdvancedFireworks/DATA/PDA_Firework.ExplosionDelay` (`self.DT_Firework`))) 2.0))
  (`NiagaraComponent.SetVariableFloat` (`self.NS_Rocket`) "Lifespan" (`self.CurrentLifespan`))
  (`NiagaraComponent.SetVariableFloat` (`self.NS_Rocket`) "RocketSpriteScale" (`/Game/AdvancedFireworks/DATA/PDA_Firework.Rocket Scale` (`self.DT_Firework`)))
  (`NiagaraComponent.SetVariableFloat` (`self.NS_Rocket`) "HueShift" (`KismetMathLibrary.RandomFloatInRange` 0.0 (`/Game/AdvancedFireworks/DATA/PDA_Firework.Rocket Hue Shift` (`self.DT_Firework`))))
  (`NiagaraComponent.SetVariableLinearColor` (`self.NS_Rocket`) "StartColor" (`/Game/AdvancedFireworks/DATA/PDA_Firework.Rocket Start Color` _dt_firework))
  (`NiagaraComponent.SetVariableLinearColor` (`self.NS_Rocket`) "EndColor" (`/Game/AdvancedFireworks/DATA/PDA_Firework.Rocket End Color` _dt_firework))
  (`NiagaraComponent.SetVariableBool` (`self.NS_Rocket`) "RandomSpriteRotation" (`/Game/AdvancedFireworks/DATA/PDA_Firework.Rocket Sprite Rotation` (`self.DT_Firework`)))
  (bind _returnvalue (`KismetMaterialLibrary.CreateDynamicMaterialInstance` "/Game/AdvancedFireworks/Materials/M_Rocket.M_Rocket"))
  (`MaterialInstanceDynamic.SetTextureParameterValue` _returnvalue "ParticleTexture" (`/Game/AdvancedFireworks/DATA/PDA_Firework.Rocket Texture` (`self.DT_Firework`)))
  (`NiagaraComponent.SetVariableMaterial` (`self.NS_Rocket`) "SpriteMaterial" _returnvalue))